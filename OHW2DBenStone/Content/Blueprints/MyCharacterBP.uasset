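; Player character Blueprint that animates a 2D survivor with a handgun using separate upper-body and lower-body flipbooks.
; A movement state enum drives UpdateAnimation, which calls per-state setters that swap flipbooks, with shooting changing only the upper body.
; Tick switches between idle and running from velocity, updating only on change; walking, strafing and shooting states are never assigned here.
; Space bar applies the running flipbooks directly without changing the state.
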(event EventBeginPlay
  (Variables|Default|SetCurMovementState "IDLE")
  (CallFunction|UpdateAnimation))

(event EventActorBeginOverlap
  (params (OtherActor :type Actor%20Object%20Reference)))

(event EventTick
  (params (DeltaSeconds :type Float%20%28single-precision%29))
  (if (> (Math|Vector|VectorLength (Transformation|GetVelocity)) 0.0)
    (if (CallFunction|NotCurState "RUNNING")
      (Variables|Default|SetCurMovementState "RUNNING")
      (CallFunction|UpdateAnimation))
    (elif (CallFunction|NotCurState "IDLE")
      (Variables|Default|SetCurMovementState "IDLE")
      (CallFunction|UpdateAnimation))))

(event Input|KeyboardEvents|SpaceBar
  (params (Key :type Key%20Structure :default "AnyKey"))
  (:Pressed
    (CallFunction|SetRunning)))

(fn ConstructionScript)

(fn SetRunning
  (Sprite|SetFlipbook (Variables|Default|GetupperBodyFB) "/Game/Sprites/Player/handgun/move/survivor-move_handgun.survivor-move_handgun")
  (Sprite|SetFlipbook (Variables|Default|GetlowerBodyFB) "/Game/Sprites/Player/feet/run/survivor-run.survivor-run"))

(fn UpdateAnimation
  (switch Utilities|FlowControl|Switch|SwitchonEMovementStates (Variables|Default|GetCurMovementState)
    (:IDLE
      (CallFunction|SetIdle))
    (:WALKING
      (CallFunction|SetWalking))
    (:RUNNING
      (CallFunction|SetRunning))
    (:STRAFE_LEFT
      (CallFunction|SetStrafeLeft))
    (:STRAFE_RIGHT
      (CallFunction|SetStrafeRight))
    (:SHOOTING
      (CallFunction|SetShooting))))

(fn SetWalking
  (Sprite|SetFlipbook (Variables|Default|GetupperBodyFB) "/Game/Sprites/Player/handgun/move/survivor-move_handgun.survivor-move_handgun")
  (Sprite|SetFlipbook (Variables|Default|GetlowerBodyFB) "/Game/Sprites/Player/feet/walk/survivor-walk.survivor-walk"))

(fn SetIdle
  (Sprite|SetFlipbook (Variables|Default|GetupperBodyFB) "/Game/Sprites/Player/handgun/idle/survivor-idle_handgun.survivor-idle_handgun")
  (Sprite|SetFlipbook (Variables|Default|GetlowerBodyFB) "/Game/Sprites/Player/feet/idle/survivor-idle.survivor-idle"))

(fn SetStrafeLeft
  (Sprite|SetFlipbook (Variables|Default|GetupperBodyFB) "/Game/Sprites/Player/handgun/move/survivor-move_handgun.survivor-move_handgun")
  (Sprite|SetFlipbook (Variables|Default|GetlowerBodyFB) "/Game/Sprites/Player/feet/strafe_left/survivor-strafe_left.survivor-strafe_left"))

(fn SetStrafeRight
  (Sprite|SetFlipbook (Variables|Default|GetupperBodyFB) "/Game/Sprites/Player/handgun/move/survivor-move_handgun.survivor-move_handgun")
  (Sprite|SetFlipbook (Variables|Default|GetlowerBodyFB) "/Game/Sprites/Player/feet/strafe_right/survivor-strafe_right.survivor-strafe_right"))

(fn SetShooting
  (Sprite|SetFlipbook (Variables|Default|GetupperBodyFB) "/Game/Sprites/Player/handgun/shoot/survivor-shoot_handgun.survivor-shoot_handgun"))

(fn NotCurState
  (params (Not%20State :type EMovementStates%20Enum))
  (return (!= (Variables|Default|GetCurMovementState) Not%20State)))